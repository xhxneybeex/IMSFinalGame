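; Rock door Blueprint that swings open once enough items have been collected.
; The collectitem event increments a counter and calls opendoor when the count reaches the maximum.
; Opendoor plays the Door timeline, whose RockDrop track lerps the static mesh's relative yaw to swing it open.
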(event `opendoor`
  (bind (_direction _rock_drop) (`Timeline|door`)
    (:`Update`
      (`SceneComponent.K2_SetRelativeRotation` (`self.StaticMesh`) (`KismetMathLibrary.MakeRotator` 0.0 0.0 (`KismetMathLibrary.Lerp` 0.0 65.0 _rock_drop)) false false))))

(event `collect item`
  (`/Engine/EditorBlueprintResources/StandardMacros.IncrementInt` (`self.currentitemscollected`)
    (:`  `
      (if (>= (`self.currentitemscollected`) (`self.maxitemscollected`))
        (`self.opendoor`)))))

(fn `UserConstructionScript`)